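; BP_Fog is a one-shot trigger actor that spawns BP_Entity in front of the player.
; On the first Trigger overlap, it casts the overlapping actor to BP_FirstPersonCharacter and spawns the entity a short distance along that actor's forward vector, owned by it.
; The look-at rotation uses a world-Y offset from the player, so it ignores player facing.
; The fog actor destroys itself after a brief delay.
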(event OnComponentBeginOverlap(Trigger)
  (params (OverlappedComponent :type Primitive%20Component%20Object%20Reference) (OtherActor :type Actor%20Object%20Reference) (OtherComp :type Primitive%20Component%20Object%20Reference) (OtherBodyIndex :type Integer) (bFromSweep :type Boolean) (SweepResult :type Hit%20Result%20Structure%20%28by%20ref%29))
  ;[0.15 0.1251 0.01934 0.5] Spawn de l'entity en face du player
  (Utilities|FlowControl|DoOnce false
    (:Completed
      (bind _asbp_first_person_character (Utilities|Casting|CastToBP_FirstPersonCharacter OtherActor))
      (Game|SpawnActorfromClass "/Game/Blueprint_ITH/BP_Entity.BP_Entity_C" (Math|Transform|MakeTransform (+ (Transformation|GetActorLocation _asbp_first_person_character) (* (Transformation|GetActorForwardVector _asbp_first_person_character) 1e+02)) (Math|Rotator|FindLookatRotation (Math|Vector|MakeVector (.x (Transformation|GetActorLocation _asbp_first_person_character)) (- (.y (Transformation|GetActorLocation _asbp_first_person_character)) 1.8e+02) (.z (Transformation|GetActorLocation _asbp_first_person_character))) (Transformation|GetActorLocation _asbp_first_person_character)) "1.000000,1.000000,1.000000") "Undefined" "MultiplyWithRoot" _asbp_first_person_character 0)
      (Utilities|FlowControl|Delay 2.0)
      (Actor|DestroyActor))))

(fn ConstructionScript)